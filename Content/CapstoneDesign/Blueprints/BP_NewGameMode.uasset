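; BP_NewGameMode is a game mode that creates the main BP_UI widget and adds it to the viewport when play begins.
; It reads the UnLockSkill flag from BP_MyGameInstance and shows or hides the skill button and character property UI to match.
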(event EventBeginPlay
  (bind _returnvalue (UserInterface|CreateWidget "/Game/CapstoneDesign/Blueprints/UI/BP_UI.BP_UI_C" 0 0))
  (bind _output_get (Variables|Default|SetUI _returnvalue))
  (UserInterface|Viewport|AddtoViewport _output_get -1)
  (bind _asbp_my_game_instance (Utilities|Casting|CastToBP_MyGameInstance (Game|GetGameInstance)))
  (if (Variables|/Script/CapstoneDesign2.MyGameInstance|GetUnLockSkill _asbp_my_game_instance)
    (Widget|SetVisibility (Variables|/Game/CapstoneDesign/Blueprints/UI/BP_UI.BP_UI_C|GetButton_Skill (Variables|Default|GetUI)) "Visible")
    (else
      (Widget|SetVisibility (Variables|/Game/CapstoneDesign/Blueprints/UI/BP_UI.BP_UI_C|GetButton_Skill (Variables|Default|GetUI)) "Hidden"))))

(fn ConstructionScript)