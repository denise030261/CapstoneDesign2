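; Game instance that holds the game's save data, loading it on Init and exposing it through GetGameData.
; LoadGameData creates a new BP_SaveGame if the slot is empty, otherwise loads asynchronously and fires OnGameLoad.
; Its synchronous load branch is unreachable because the existence check is repeated.
; SavePlayer stores player data in the save object and calls SaveGameData, which writes synchronously or asynchronously.
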(event EventInit
  (CallFunction|LoadGameData false))

(event EventSaveGameData
  (params (Async :type Boolean))
  ;[1 1 1] Save Game
  (if Async
    (|AsyncSaveGametoSlot (Variables|Default|GetSavedData) (Variables|Default|GetSlotName))
    (else
      (SaveGame|SaveGametoSlot (Variables|Default|GetSavedData) (Variables|Default|GetSlotName)))))

(event EventLoadGameData
  (params (Async :type Boolean))
  ;[1 1 1] LoadGame
  (bind _returnvalue (SaveGame|DoesSaveGameExist (Variables|Default|GetSlotName)))
  (if _returnvalue
    (if _returnvalue
      (bind _savegame (|AsyncLoadGamefromSlot (Variables|Default|GetSlotName))
        (:Completed
          (bind _asbp_save_game (Utilities|Casting|CastToBP_SaveGame _savegame))
          (Variables|Default|SetSavedData _asbp_save_game)
          (Default|CallOnGameLoad)))
      (else
        (bind _returnvalue_2 (SaveGame|LoadGamefromSlot (Variables|Default|GetSlotName)))
        (bind _asbp_save_game_2 (Utilities|Casting|CastToBP_SaveGame _returnvalue_2))
        (Variables|Default|SetSavedData _asbp_save_game_2)))
    (else
      (bind _returnvalue_3 (SaveGame|CreateSaveGameObject "/Game/CapstoneDesign/Blueprints/Save/BP_SaveGame.BP_SaveGame_C"))
      (Variables|Default|SetSavedData _returnvalue_3))))

(event EventSavePlayer
  (params (PlayerSave :type S%20Player%20Save%20Structure) (Async :type Boolean))
  (Variables|/Game/CapstoneDesign/Blueprints/Save/BP_SaveGame.BP_SaveGame_C|SetPlayerSave (Variables|Default|GetSavedData) PlayerSave)
  (CallFunction|SaveGameData Async))

(fn GetGameData
  (return (Variables|Default|GetSavedData)))