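; Player character that paints on canvases, talks to nearby NPCs and a pot, and switches its attribute.
; Paint input traces from the cursor and passes the hit UV, brush texture and size to Canvas_BP to draw.
; A gamepad axis moves the mouse cursor.
; R or the gamepad bottom button calls TalkMessage through BPI_Dialogue on overlapping actors, while Z and C set CurAttribute to Normal or Fire.
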(event Input|EnhancedActionEvents|EnhancedInputActionIA_Paint
  (params (ActionValue :type Float%20%28double-precision%29) (ElapsedSeconds :type Float%20%28double-precision%29) (TriggeredSeconds :type Float%20%28double-precision%29) (InputAction :type Input%20Action%20Object%20Reference :default "/Game/CapstoneDesign/Input/IA_Paint.IA_Paint"))
  (bind _returnvalue (Game|GetPlayerController 0))
  (bind (_worldlocation _worlddirection) (Game|Player|ConvertMouseLocationToWorldSpace _returnvalue))
  (if (== ActionValue 1.0)
    (bind _outhit (Collision|LineTraceByChannel _worldlocation (+ _worldlocation (* _worlddirection 2e+03)) "TraceTypeQuery1" true 0 "None"))
    (bind _ascanvas_bp (Utilities|Casting|CastToCanvas_BP (.HitActor (Collision|BreakHitResult _outhit))))
    (Default|Drawbrush _ascanvas_bp (Variables|Default|GetBrushtexture) (Variables|Default|GetBrushsize) (.UV (Class|GameplayStatics|FindCollisionUV _outhit)))))

(event Input|EnhancedActionEvents|EnhancedInputActionIA_GamePadMouse
  (params (ActionValue :type Vector%202D%20Structure) (ElapsedSeconds :type Float%20%28double-precision%29) (TriggeredSeconds :type Float%20%28double-precision%29) (InputAction :type Input%20Action%20Object%20Reference :default "/Game/CapstoneDesign/Input/IA_GamePadMouse.IA_GamePadMouse"))
  (bind _returnvalue (Utilities|Time|GetWorldDeltaSeconds))
  (bind _returnvalue_2 (Game|GetPlayerController 0))
  (bind (_locationx _locationy) (Game|Player|GetMousePosition _returnvalue_2))
  (bind _returnvalue_3 (* ActionValue _returnvalue 1e+03))
  (Class|PlayerController|SetMouseLocation _returnvalue_2 (Math|Float|Truncate (+ _locationx (.x _returnvalue_3))) (Math|Float|Truncate (+ _locationy (.y _returnvalue_3)))))

(event EventBeginPlay
  (Pawn|SpawnDefaultController)
  (Input|SetInputModeGameOnly (Game|GetPlayerController 0) true))

(event Input|GamepadEvents|GamepadFaceButtonBottom
  (params (Key :type Key%20Structure :default "None"))
  (:Pressed
    (for _array_element (Collision|GetOverlappingActors "/Game/CapstoneDesign/Blueprints/NPC/BP_Pot.BP_Pot_C" :!class /Script/Engine.Actor)
      (if (Utilities|DoesObjectImplementInterface _array_element "/Game/CapstoneDesign/Blueprints/NPC/BPI_Dialogue.BPI_Dialogue_C")
        (Class|BPIDialogue|Talk(Message) _array_element)))))

(event Input|KeyboardEvents|Z
  (params (Key :type Key%20Structure :default "None"))
  (:Pressed
    (Variables|Default|SetCurAttribute "Normal")))

(event Input|KeyboardEvents|C
  (params (Key :type Key%20Structure :default "None"))
  (:Pressed
    (Variables|Default|SetCurAttribute "Fire")))

(event Input|KeyboardEvents|R
  (params (Key :type Key%20Structure :default "None"))
  (:Pressed
    (for _array_element (Collision|GetOverlappingActors "/Game/CapstoneDesign/Blueprints/NPC/BP_Pot.BP_Pot_C" :!class /Script/Engine.Actor)
      (if (Utilities|DoesObjectImplementInterface _array_element "/Game/CapstoneDesign/Blueprints/NPC/BPI_Dialogue.BPI_Dialogue_C")
        (Class|BPIDialogue|Talk(Message) _array_element)))))

(event Input|KeyboardEvents|R
  (params (Key :type Key%20Structure :default "None"))
  (:Pressed
    (for _array_element (Collision|GetOverlappingActors "/Game/CapstoneDesign/Blueprints/NPC/BP_NPC1.BP_NPC1_C" :!class /Script/Engine.Actor)
      (if (Utilities|DoesObjectImplementInterface _array_element "/Game/CapstoneDesign/Blueprints/NPC/BPI_Dialogue.BPI_Dialogue_C")
        (Class|BPIDialogue|Talk(Message) _array_element)))))

(event Input|GamepadEvents|GamepadFaceButtonBottom
  (params (Key :type Key%20Structure :default "None"))
  (:Pressed
    (for _array_element (Collision|GetOverlappingActors "/Game/CapstoneDesign/Blueprints/NPC/BP_NPC1.BP_NPC1_C" :!class /Script/Engine.Actor)
      (if (Utilities|DoesObjectImplementInterface _array_element "/Game/CapstoneDesign/Blueprints/NPC/BPI_Dialogue.BPI_Dialogue_C")
        (Class|BPIDialogue|Talk(Message) _array_element)))))

(event Input|KeyboardEvents|R
  (params (Key :type Key%20Structure :default "None"))
  (:Pressed
    (Development|PrintString "Hello")
    (for _array_element (Collision|GetOverlappingActors "/Game/CapstoneDesign/Blueprints/NPC/BP_NPC2.BP_NPC2_C" :!class /Script/Engine.Actor)
      (if (Utilities|DoesObjectImplementInterface _array_element "/Game/CapstoneDesign/Blueprints/NPC/BPI_Dialogue.BPI_Dialogue_C")
        (Class|BPIDialogue|Talk(Message) _array_element)))))

(event Input|GamepadEvents|GamepadFaceButtonBottom
  (params (Key :type Key%20Structure :default "None"))
  (:Pressed
    (Development|PrintString "Hello")
    (for _array_element (Collision|GetOverlappingActors "/Game/CapstoneDesign/Blueprints/NPC/BP_NPC2.BP_NPC2_C" :!class /Script/Engine.Actor)
      (if (Utilities|DoesObjectImplementInterface _array_element "/Game/CapstoneDesign/Blueprints/NPC/BPI_Dialogue.BPI_Dialogue_C")
        (Class|BPIDialogue|Talk(Message) _array_element)))))

(fn ConstructionScript)