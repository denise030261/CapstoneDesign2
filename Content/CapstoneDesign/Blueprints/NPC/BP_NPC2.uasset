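; Quest NPC for a troubled villager who asks the player to find lost iron pieces, with a name widget set on BeginPlay.
; Each Talk call steps through quest or completion dialogue, chosen by the GameInstance iron count, in a viewport widget with sound and haptics.
; Set lines update the quest string and fire quest events; the main input mapping is removed during dialogue and restored afterward.
; Trigger-zone overlaps only log.
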(event OnComponentBeginOverlap(TriggerZone)
  (params (OverlappedComponent :type Primitive%20Component%20Object%20Reference) (OtherActor :type Actor%20Object%20Reference) (OtherComp :type Primitive%20Component%20Object%20Reference) (OtherBodyIndex :type Integer) (bFromSweep :type Boolean) (SweepResult :type Hit%20Result%20Structure%20%28by%20ref%29))
  (Utilities|Casting|CastToBP_MainCharacter OtherActor)
  (Utilities|String|LogString "start"))

(event OnComponentEndOverlap(TriggerZone)
  (params (OverlappedComponent :type Primitive%20Component%20Object%20Reference) (OtherActor :type Actor%20Object%20Reference) (OtherComp :type Primitive%20Component%20Object%20Reference) (OtherBodyIndex :type Integer))
  (Utilities|Casting|CastToBP_MainCharacter OtherActor)
  (Utilities|String|LogString "end"))

(event EventBeginPlay
  (bind _returnvalue (UserInterface|CreateWidget "/Game/CapstoneDesign/Blueprints/NPC/NPC_UI.NPC_UI_C"))
  (bind _output_get (Variables|Default|SetNPC_UI _returnvalue))
  (Default|NPCsetName _output_get "곤란해하는 주민")
  (UserInterface|SetWidget (Variables|Default|GetWidget) _output_get))

(event EventTalk
  (bind _returnvalue (Game|GetPlayerController 0))
  (bind _returnvalue_2 (Game|GetPlayerController 0))
  (bind _returnvalue_3 (PlayerController|LocalPlayerSubsystems|GetEnhancedInputLocalPlayerSubsystem _returnvalue))
  (Input|RemoveMappingContext _returnvalue_3 "/Game/CapstoneDesign/Input/IMC_MainCharacter.IMC_MainCharacter" "(bIgnoreAllPressedKeysUntilRelease=True,bForceImmediately=False,bNotifyUserSettings=False)")
  (Input|EnableInput _returnvalue 0)
  (bind _asmy_game_instance (Utilities|Casting|CastToMyGameInstance (Game|GetGameInstance)))
  (Variables|Default|Set%20Game%20Instance _asmy_game_instance)
  (bind _output_get (Variables|Default|SetQuestComplete (>= (Variables|/Script/CapstoneDesign2.MyGameInstance|GetIronCount (Variables|Default|Get%20Game%20Instance)) 3)))
  (if _output_get
    (Variables|/Script/CapstoneDesign2.MyGameInstance|SetGetNPC2Quest (Variables|Default|Get%20Game%20Instance) false)
    (Variables|Default|SetQuestComplete true)
    (Math|Integer|IncrementInt (Variables|Default|GetCompleteIndex)
      (:%20%20
        (if (< (Variables|Default|GetCompleteIndex) (Utilities|Array|Length (Variables|Default|GetCompleteText)))
          (Variables|Default|GetTalkNPC
            (:then
              _)
            (:else
              (bind _returnvalue_4 (UserInterface|CreateWidget "/Game/CapstoneDesign/Blueprints/NPC/WB_TalkNPC.WB_TalkNPC_C" (Game|GetPlayerController 0)))
              (bind _output_get_2 (Variables|Default|SetTalkNPC _returnvalue_4))
              (UserInterface|Viewport|AddtoViewport _output_get_2 0)))
          (Rendering|Components|TextRender|SetText (Variables|/Game/CapstoneDesign/Blueprints/NPC/WB_TalkNPC.WB_TalkNPC_C|GetNPCTalkText (Variables|Default|GetTalkNPC)) (Utilities|Text|ToText(String) (Utilities|Array|Get(acopy) (Variables|Default|GetCompleteText) (Variables|Default|GetCompleteIndex))))
          (Audio|PlaySound2D "/Engine/EngineSounds/1kSineTonePing.1kSineTonePing" 1.0 1.0 0.0 0 0)
          (Game|Feedback|ClientPlayForceFeedback (Game|GetPlayerController 0) "/Game/CapstoneDesign/Input/ForceFeedback/UIForceFeedbackEffect.UIForceFeedbackEffect" "None" false false false)
          (if (== (Variables|Default|GetCompleteIndex) 2)
            (bind _asbp_my_game_instance (Utilities|Casting|CastToBP_MyGameInstance (Game|GetGameInstance)))
            (Class|MyGameInstance|SetQuestString _asbp_my_game_instance "부엌에 가서 음식 먹기")
            (Default|CallCompleteQuestNPC2))
          (else
            (Widget|RemovefromParent (Variables|Default|GetTalkNPC))
            (Components|DestroyComponent (Variables|Default|GetnotifyNPC))
            (Input|AddMappingContext _returnvalue_3 "/Game/CapstoneDesign/Input/IMC_MainCharacter.IMC_MainCharacter" 0 "(bIgnoreAllPressedKeysUntilRelease=True,bForceImmediately=False,bNotifyUserSettings=False)" :!label _label)
            (Input|DisableInput _returnvalue_2 0)))))
    (else
      (Variables|/Script/CapstoneDesign2.MyGameInstance|SetGetNPC2Quest (Variables|Default|Get%20Game%20Instance) true)
      (Math|Integer|IncrementInt (Variables|Default|GettalkIndex)
        (:%20%20
          (if (< (Variables|Default|GettalkIndex) (Utilities|Array|Length (Variables|Default|Getdialogue)))
            (Variables|Default|GetTalkNPC
              (:then
                _)
              (:else
                (bind _returnvalue_5 (UserInterface|CreateWidget "/Game/CapstoneDesign/Blueprints/NPC/WB_TalkNPC.WB_TalkNPC_C" _returnvalue_2))
                (bind _output_get_3 (Variables|Default|SetTalkNPC _returnvalue_5))
                (UserInterface|Viewport|AddtoViewport _output_get_3 0)))
            (Rendering|Components|TextRender|SetText (Variables|/Game/CapstoneDesign/Blueprints/NPC/WB_TalkNPC.WB_TalkNPC_C|GetNPCTalkText (Variables|Default|GetTalkNPC)) (Utilities|Text|ToText(String) (Utilities|Array|Get(acopy) (Variables|Default|Getdialogue) (Variables|Default|GettalkIndex))))
            (Audio|PlaySound2D "/Engine/EngineSounds/1kSineTonePing.1kSineTonePing" 1.0 1.0 0.0 0 0)
            (Game|Feedback|ClientPlayForceFeedback (Game|GetPlayerController 0) "/Game/CapstoneDesign/Input/ForceFeedback/UIForceFeedbackEffect.UIForceFeedbackEffect" "None" false false false)
            (if (== (Variables|Default|GettalkIndex) 4)
              (bind _asbp_my_game_instance_2 (Utilities|Casting|CastToBP_MyGameInstance (Game|GetGameInstance)))
              (Class|MyGameInstance|SetQuestString _asbp_my_game_instance_2 "숲속에서 잃어버린 쇠붙이 찾기")
              (Default|CallEncountandEndTalkNPC2))
            (else
              (Widget|RemovefromParent (Variables|Default|GetTalkNPC))
              (goto _label))))))))

(fn ConstructionScript)