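; BP_Pot is an interactable pot that toggles the paintbrush UI.
; The R key, the gamepad bottom face button and the Talk event share one toggle driven by IsWidget.
; Opening finds the Canvas_BP actor, passes it to a new Paintbrush_wbp as Target, shows the cursor and sets Game-and-UI input.
; Closing removes the widget, hides the cursor and restores game-only input.
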(event EventTalk
  (bind _returnvalue (Game|GetPlayerController 0))
  (if (Variables|Default|GetIsWidget)
    (Variables|Default|SetIsWidget false)
    (Widget|RemovefromParent (stale _returnvalue_3))
    (Input|SetInputModeGameOnly _returnvalue false)
    (Variables|/Script/Engine.PlayerController|SetbShowMouseCursor _returnvalue false)
    (else
      (bind _returnvalue_2 (Actor|GetActorOfClass "/Game/CapstoneDesign/Blueprints/UI/Canvas_BP.Canvas_BP_C"))
      (bind _returnvalue_3 (UserInterface|CreateWidget "/Game/CapstoneDesign/Blueprints/UI/Paintbrush_wbp.Paintbrush_wbp_C" 0 _returnvalue_2))
      (bind _output_get (Variables|Default|SetNewVar _returnvalue_3))
      (UserInterface|Viewport|AddtoViewport _returnvalue_3 0)
      (Variables|Default|SetIsWidget true)
      (Input|SetInputModeGameandUI _returnvalue 0 "DoNotLock" true false)
      (Variables|/Script/Engine.PlayerController|SetbShowMouseCursor _returnvalue true))))

(event Input|GamepadEvents|GamepadFaceButtonBottom
  (params (Key :type Key%20Structure :default "None"))
  (bind _returnvalue (Game|GetPlayerController 0))
  (:Pressed
    (if (Variables|Default|GetIsWidget)
      (Variables|Default|SetIsWidget false)
      (Widget|RemovefromParent (stale _returnvalue_3))
      (Input|SetInputModeGameOnly _returnvalue false)
      (Variables|/Script/Engine.PlayerController|SetbShowMouseCursor _returnvalue false)
      (else
        (bind _returnvalue_2 (Actor|GetActorOfClass "/Game/CapstoneDesign/Blueprints/UI/Canvas_BP.Canvas_BP_C"))
        (bind _returnvalue_3 (UserInterface|CreateWidget "/Game/CapstoneDesign/Blueprints/UI/Paintbrush_wbp.Paintbrush_wbp_C" 0 _returnvalue_2))
        (bind _output_get (Variables|Default|SetNewVar _returnvalue_3))
        (UserInterface|Viewport|AddtoViewport _returnvalue_3 0)
        (Variables|Default|SetIsWidget true)
        (Input|SetInputModeGameandUI _returnvalue 0 "DoNotLock" true false)
        (Variables|/Script/Engine.PlayerController|SetbShowMouseCursor _returnvalue true)))))

(event Input|KeyboardEvents|R
  (params (Key :type Key%20Structure :default "None"))
  (bind _returnvalue (Game|GetPlayerController 0))
  (:Pressed
    (if (Variables|Default|GetIsWidget)
      (Variables|Default|SetIsWidget false)
      (Widget|RemovefromParent (stale _returnvalue_3))
      (Input|SetInputModeGameOnly _returnvalue false)
      (Variables|/Script/Engine.PlayerController|SetbShowMouseCursor _returnvalue false)
      (else
        (bind _returnvalue_2 (Actor|GetActorOfClass "/Game/CapstoneDesign/Blueprints/UI/Canvas_BP.Canvas_BP_C"))
        (bind _returnvalue_3 (UserInterface|CreateWidget "/Game/CapstoneDesign/Blueprints/UI/Paintbrush_wbp.Paintbrush_wbp_C" 0 _returnvalue_2))
        (bind _output_get (Variables|Default|SetNewVar _returnvalue_3))
        (UserInterface|Viewport|AddtoViewport _returnvalue_3 0)
        (Variables|Default|SetIsWidget true)
        (Input|SetInputModeGameandUI _returnvalue 0 "DoNotLock" true false)
        (Variables|/Script/Engine.PlayerController|SetbShowMouseCursor _returnvalue true)))))

(fn ConstructionScript)