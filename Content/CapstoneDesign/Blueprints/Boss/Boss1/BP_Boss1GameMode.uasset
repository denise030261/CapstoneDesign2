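; Game mode for the first boss fight that sets up the stage and its HUD on BeginPlay.
; A constructed Boss1GameModeHelper runs SetStage after the parent BeginPlay and supplies the Boss1 reference to the boss UI widget.
; The boss UI and the general UI, owned by the first player controller, are then added to the viewport.
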(event EventBeginPlay
  (bind _returnvalue (Game|ConstructObjectfromClass "/Script/CapstoneDesign2.Boss1GameModeHelper"))
  (|CallParentFunction)
  (Class|Boss1GameModeHelper|SetStage _returnvalue)
  (bind _returnvalue_2 (UserInterface|CreateWidget "/Game/CapstoneDesign/Blueprints/Boss/Boss1/BP_Boss1UI.BP_Boss1UI_C"))
  (Variables|/Script/CapstoneDesign2.Boss1UI|SetBoss1 _returnvalue_2 (Variables|/Script/CapstoneDesign2.Boss1GameModeHelper|GetBoss1 _returnvalue))
  (UserInterface|Viewport|AddtoViewport _returnvalue_2 0)
  (bind _returnvalue_3 (UserInterface|CreateWidget "/Game/CapstoneDesign/Blueprints/UI/BP_UI.BP_UI_C" (Game|GetPlayerController 0) 0))
  (UserInterface|Viewport|AddtoViewport _returnvalue_3 0))

(event EventTick
  (params (DeltaSeconds :type Float%20%28single-precision%29))
  (|CallParentFunction DeltaSeconds) ; 지금 이 노드는 비활성 상태입니다. \n핀을 끌어서 다른 노드를 연결하면 활성화됩니다.
)

(fn ConstructionScript
  (|CallParentFunction))